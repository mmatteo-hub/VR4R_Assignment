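; Node actor with a sphere whose color shows how recently a flying drone pawn was nearby.
; Each tick it checks every BP_FlyingPawn and records the real time whenever one is within a fixed radius.
; Inside that loop, the sphere material's Color parameter lerps from green to red as time since that last visit approaches ColorResetTime.
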(event `self.ReceiveTick`
  (params (DeltaSeconds :type "Float (single-precision)"))
  (bind _outactors (`GameplayStatics.GetAllActorsOfClass` "/AirSim/Blueprints/BP_FlyingPawn.BP_FlyingPawn_C"))
  (for _array_element _outactors
    (if (< (`self.GetDistanceTo` _array_element) 250.0)
      (set `self.TimeAtDroneLeave` (`GameplayStatics.GetRealTimeSeconds`)))
    (`MeshComponent.SetVectorParameterValueOnMaterials` (`self.Sphere`) "Color" (`KismetMathLibrary.VLerp` (0.0 1.0 0.0) (1.0 0.0 0.0) (`KismetMathLibrary.FClamp` (/ (- (`GameplayStatics.GetRealTimeSeconds`) (`self.TimeAtDroneLeave`)) (`self.ColorResetTime`)))))))

(fn `UserConstructionScript`)